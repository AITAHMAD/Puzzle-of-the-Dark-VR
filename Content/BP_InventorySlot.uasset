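; Inventory slot actor that stores one grabbable actor released inside its overlap sphere.
; Overlap binds to GrabComponent grab and drop events and enlarges the Sphere as a highlight, resetting it on drop or exit.
; Dropping into an empty slot disables physics, attaches the actor and rescales it relative to the sphere.
; Grabbing or overlap exit releases it at its saved scale; exit unbinding searches the slot's own components, not the leaving actor's.
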(event `self.ReceiveBeginPlay`
  (set `self.InitialSellScale` (`SceneComponent.K2_GetComponentScale` (`self.Sphere`))))

(event `self.Sphere1.OnComponentBeginOverlap`
  (params (OverlappedComponent :type "PrimitiveComponent Object Reference") (OtherActor :type "Actor Object Reference") (OtherComp :type "PrimitiveComponent Object Reference") (OtherBodyIndex :type Integer) (bFromSweep :type Boolean) (SweepResult :type "HitResult Structure (by ref)"))
  (for _array_element (`self.K2_GetComponentsByClass` OtherActor "/Game/VRTemplate/Blueprints/GrabComponent.GrabComponent_C")
    (`KismetArrayLibrary.Array_Add` (`self.TrackedGrabComponents`) _array_element)
    (add `/Game/VRTemplate/Blueprints/GrabComponent.OnGrabbed` _array_element (delegate `OnGrabbed_Event`))
    (add `/Game/VRTemplate/Blueprints/GrabComponent.OnDropped` _array_element (delegate `OnDropped_Event`)))
  (`self.IncreaseCellSize`))

(event `OnGrabbed_Event`
  (params (`Self Reference` :type "/Game/VRTemplate/Blueprints/GrabComponent Object Reference"))
  (`self.TryDropObject` (`ActorComponent.GetOwner` `Self Reference`)))

(event `OnDropped_Event`
  (params (`Self Reference` :type "/Game/VRTemplate/Blueprints/GrabComponent Object Reference"))
  (`self.TryCaptureObject` `Self Reference`)
  (`self.DecreasecellSize`))

(event `self.Sphere1.OnComponentEndOverlap`
  (params (OverlappedComponent :type "PrimitiveComponent Object Reference") (OtherActor :type "Actor Object Reference") (OtherComp :type "PrimitiveComponent Object Reference") (OtherBodyIndex :type Integer))
  (`self.TryDropObject` OtherActor)
  (for _array_element (`self.K2_GetComponentsByClass` "/Game/VRTemplate/Blueprints/GrabComponent.GrabComponent_C")
    (`KismetArrayLibrary.Array_RemoveItem` (`self.TrackedGrabComponents`) _array_element)
    (remove `/Game/VRTemplate/Blueprints/GrabComponent.OnGrabbed` _array_element (delegate `OnGrabbed_Event`))
    (remove `/Game/VRTemplate/Blueprints/GrabComponent.OnDropped` _array_element (delegate `OnDropped_Event`)))
  (`self.DecreasecellSize`))

(fn `DecreasecellSize`
  (`SceneComponent.SetWorldScale3D` (`self.Sphere`) (`self.InitialSellScale`)))

(fn `IncreaseCellSize`
  (`SceneComponent.SetWorldScale3D` (`self.Sphere`) (* (`self.InitialSellScale`) 1.2)))

(fn `TryCaptureObject`
  (params (`Grab component` :type "/Game/VRTemplate/Blueprints/GrabComponent Object Reference"))
  (`/Engine/EditorBlueprintResources/StandardMacros.IsValid` (`self.HeldActor`)
    (:`Is Not Valid`
      (bind _output_get (set `self.HeldActor` (`ActorComponent.GetOwner` `Grab component`)))
      (set `self.InitialActorScale` (`self.GetActorScale3D` _output_get))
      (`/Game/VRTemplate/Blueprints/GrabComponent.SetPrimitiveCompPhysics` `Grab component` false)
      (`self.K2_AttachToComponent` _output_get (`self.DefaultSceneRoot`) "None" "SnapToTarget" "KeepWorld" "KeepWorld" true)
      (`self.SetActorScale3D` (`self.HeldActor`) (* (`self.InitialSellScale`) 0.5)))))

(fn `TryDropObject`
  (params (Actor :type "Actor Object Reference"))
  (bind _heldactor (`self.HeldActor`))
  (`/Engine/EditorBlueprintResources/StandardMacros.IsValid` _heldactor
    (:`Is Valid`
      (if (== Actor _heldactor)
        (if (== (`self.GetAttachParentActor` (`self.HeldActor`)) self)
          (`self.K2_DetachFromActor` (`self.HeldActor`) "KeepRelative" "KeepRelative" "KeepRelative"))
        (`self.SetActorScale3D` (`self.HeldActor`) (`self.InitialActorScale`))
        (set `self.HeldActor` null)))))

(fn `UserConstructionScript`)